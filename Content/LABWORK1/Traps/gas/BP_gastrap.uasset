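; BP_gastrap is a gas trap that deals repeated damage to the third-person character inside its collision sphere.
; The gas cloud is made visible at BeginPlay and again on each overlap.
; Overlap start sets IsInside before casting to the character, then a Delay loop applies small damage every half second while the flag holds.
; Any overlap end clears the flag, without checking which actor left.
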(event OnComponentBeginOverlap(Spherecollisio)
  (params (OverlappedComponent :type Primitive%20Component%20Object%20Reference) (OtherActor :type Actor%20Object%20Reference) (OtherComp :type Primitive%20Component%20Object%20Reference) (OtherBodyIndex :type Integer) (bFromSweep :type Boolean) (SweepResult :type Hit%20Result%20Structure%20%28by%20ref%29))
  (Rendering|SetVisibility (Variables|Default|Getgascloud1) true false)
  (Variables|Default|SetisInside true)
  (bind _asbp_third_person_character (Utilities|Casting|CastToBP_ThirdPersonCharacter OtherActor))
  (Game|Damage|ApplyDamage _asbp_third_person_character 2.0 0 0 :!label _label)
  (if (Variables|Default|GetisInside)
    (Utilities|FlowControl|Delay 0.5)
    (goto _label)))

(event OnComponentEndOverlap(Spherecollisio)
  (params (OverlappedComponent :type Primitive%20Component%20Object%20Reference) (OtherActor :type Actor%20Object%20Reference) (OtherComp :type Primitive%20Component%20Object%20Reference) (OtherBodyIndex :type Integer))
  (Variables|Default|SetisInside false))

(event EventBeginPlay
  (Rendering|SetVisibility (Variables|Default|Getgascloud1) true false))

(event Collision|EventActorBeginOverlap
  (params (OtherActor :type Actor%20Object%20Reference)))

(event EventTick
  (params (DeltaSeconds :type Float%20%28single-precision%29)))

(fn ConstructionScript)
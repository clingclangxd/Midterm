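; BP_Axe is an axe trap that stays hidden until something overlaps its Wireline trigger.
; On trigger, it reveals the axe and plays a timeline that swings it by scaling the Rotation track into relative pitch.
; A separate AxeColl overlap applies fixed damage to BP_ThirdPersonCharacter, with no check that the trap has been triggered.
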(event OnComponentBeginOverlap(wireline)
  (params (OverlappedComponent :type Primitive%20Component%20Object%20Reference) (OtherActor :type Actor%20Object%20Reference) (OtherComp :type Primitive%20Component%20Object%20Reference) (OtherBodyIndex :type Integer) (bFromSweep :type Boolean) (SweepResult :type Hit%20Result%20Structure%20%28by%20ref%29))
  (Rendering|SetVisibility (Variables|Default|GetAxe) true false)
  (bind _rotation (Timeline|Timeline Play)
    (:Update
      (Transformation|SetRelativeRotation (Variables|Default|GetAxe) (Math|Rotator|MakeRotator 0.0 (* _rotation 7e+01) 0.0) false false))))

(event OnComponentBeginOverlap(AxeColl)
  (params (OverlappedComponent :type Primitive%20Component%20Object%20Reference) (OtherActor :type Actor%20Object%20Reference) (OtherComp :type Primitive%20Component%20Object%20Reference) (OtherBodyIndex :type Integer) (bFromSweep :type Boolean) (SweepResult :type Hit%20Result%20Structure%20%28by%20ref%29))
  (bind _asbp_third_person_character (Utilities|Casting|CastToBP_ThirdPersonCharacter OtherActor))
  (Game|Damage|ApplyDamage _asbp_third_person_character 2e+01 0 0))

(event EventBeginPlay
  (Rendering|SetVisibility (Variables|Default|GetAxe) false false))

(event Collision|EventActorBeginOverlap
  (params (OtherActor :type Actor%20Object%20Reference)))

(event EventTick
  (params (DeltaSeconds :type Float%20%28single-precision%29)))

(fn ConstructionScript)